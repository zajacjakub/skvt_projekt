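; Player controller for Skvt that sets up Enhanced Input and manages HUD, pause menu and move-tutorial widgets.
; BeginPlay adds the default and swap-pawn mapping contexts, then spawns the HUD.
; IA_OpenMenu toggles the main menu with pause, cursor and input mode; IA_Move hides the tutorial or clears its timer.
; Character cycling through possession and the tutorial's start timer exist but are unwired, so neither runs.
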(event Custom|ShowMoveTutorial
  (bind _returnvalue (UserInterface|CreateWidget "/Game/Skvt/UI/Widgets/Tutorial/WBP_MoveTutorial.WBP_MoveTutorial_C" self))
  (bind _output_get (Variables|Tutorial|SetMoveTutorialWidget _returnvalue))
  (UserInterface|Viewport|AddtoViewport _output_get 0))

(event Custom|HideMoveTutorial
  (Widget|RemovefromParent (Variables|Tutorial|GetMoveTutorialWidget)))

(event Input|EnhancedActionEvents|EnhancedInputActionIA_OpenMenu
  (params (ActionValue :type Boolean) (ElapsedSeconds :type Float%20%28double-precision%29) (TriggeredSeconds :type Float%20%28double-precision%29) (InputAction :type Input%20Action%20Object%20Reference :default "/Game/Skvt/Characters/Input/Actions/IA_OpenMenu.IA_OpenMenu"))
  (:Triggered
    (Utilities|IsValid (Variables|Default|GetMainMenuWidget)
      (:Is%20Valid
        (CallFunction|CloseMainMenu))
      (:Is%20Not%20Valid
        (CallFunction|OpenMainMenu)))))

(event Input|EnhancedActionEvents|EnhancedInputActionIA_Move
  (params (ActionValue :type Vector%202D%20Structure) (ElapsedSeconds :type Float%20%28double-precision%29) (TriggeredSeconds :type Float%20%28double-precision%29) (InputAction :type Input%20Action%20Object%20Reference :default "/Game/ThirdPerson/Input/Actions/IA_Move.IA_Move"))
  (:Triggered
    (Utilities|IsValid (Variables|Tutorial|GetMoveTutorialWidget)
      (:Is%20Valid
        (CallFunction|HideMoveTutorial))
      (:Is%20Not%20Valid
        (Utilities|Time|ClearandInvalidateTimerbyHandle (Variables|Tutorial|GetMoveTutorialTimer))))))

(event EventBeginPlay
  (CallFunction|AddInputMappings)
  (Utilities|FlowControl|Sequence
    (:then_0
      (CallFunction|SpawnPlayerHUD))))

(fn ConstructionScript)

(fn SelectCharactertoPossess
  (bind _outactors (Actor|GetAllActorsOfClass "/Game/Skvt/Characters/BP_SkvtBaseChar.BP_SkvtBaseChar_C"))
  (bind _output_get (LocalVariables|SetChacters _outactors))
  (if (< (+ (Utilities|Array|FindItem _output_get 0) 1) (Utilities|Array|Length _output_get))
    (return (Utilities|Array|Get(acopy) (LocalVariables|GetChacters) (+ (Utilities|Array|FindItem _output_get 0) 1)))
    (else
      (return (Utilities|Array|Get(acopy) (LocalVariables|GetChacters))))))

(fn OpenMainMenu
  (bind _returnvalue (UserInterface|CreateWidget "/Game/Skvt/UI/Widgets/Menu/WBP_MainMenu.WBP_MainMenu_C" self))
  (bind _output_get (Variables|Default|SetMainMenuWidget _returnvalue))
  (UserInterface|Viewport|AddtoViewport _output_get 0)
  (Input|SetInputModeGameandUI self 0 "DoNotLock" true false)
  (Variables|Default|SetbShowMouseCursor true)
  (Game|SetGamePaused true))

(fn CloseMainMenu
  (Widget|RemovefromParent (Variables|Default|GetMainMenuWidget))
  (Variables|Default|SetMainMenuWidget 0)
  (Input|SetInputModeGameOnly self false)
  (Variables|Default|SetbShowMouseCursor false)
  (Game|SetGamePaused false))

(fn AddInputMappings
  (bind _self self)
  (bind _returnvalue (PlayerController|LocalPlayerSubsystems|GetEnhancedInputLocalPlayerSubsystem _self))
  (Utilities|IsValid _returnvalue
    (:Is%20Valid
      (Input|AddMappingContext _returnvalue "/Game/ThirdPerson/Input/IMC_Default.IMC_Default" 0 "(bIgnoreAllPressedKeysUntilRelease=True,bForceImmediately=False)")
      (Input|AddMappingContext _returnvalue "/Game/Skvt/Characters/Input/IMC_SwapPawn.IMC_SwapPawn" 0 "(bIgnoreAllPressedKeysUntilRelease=True,bForceImmediately=False)"))))

(fn SpawnPlayerHUD
  (bind _returnvalue (UserInterface|CreateWidget "/Game/Skvt/UI/Widgets/HUD/WBP_HUD.WBP_HUD_C" self))
  (bind _output_get (Variables|Default|SetHUDWidget _returnvalue))
  (UserInterface|Viewport|AddtoViewport _output_get 0))