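; Base NPC character that takes damage, dies, and can be taken down by the player through interaction.
; Damage feeds the health component and plays a hit montage; its death event enables mesh ragdoll physics, then destroys the actor after a delay.
; Takedown marks the NPC dead, snaps the player behind it, plays paired neck-break montages, then restores only the player's movement.
; The offered interaction action depends on the dead flag.
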(event OnDeath(BP_HealthComponent)
  (Pawn|Components|CharacterMovement|DisableMovement (Variables|Character|GetCharacterMovement))
  (Physics|SetSimulatePhysics (Variables|Character|GetMesh) true)
  (Utilities|Time|SetTimerbyEvent (delegate Custom|FinalizeDeath) 5.0))

(event Custom|FinalizeDeath
  (Actor|DestroyActor))

(event Custom|Takedown
  (params (NewParam :type Boolean))
  (bind _returnvalue (Transformation|GetActorTransform))
  (Variables|Default|SetIsDead true)
  (Default|UpdateInteractWidget (Variables|Default|GetPlayerCharacter))
  (Pawn|Components|CharacterMovement|DisableMovement (Variables|Character|GetCharacterMovement))
  (Pawn|Components|CharacterMovement|DisableMovement (Variables|/Script/Engine.Character|GetCharacterMovement (Variables|Default|GetPlayerCharacter)))
  (Transformation|SetActorTransform (Variables|Default|GetPlayerCharacter) (Math|Transform|MakeTransform (+ (.location _returnvalue) (* (Transformation|GetActorForwardVector) -1.1e+02)) (.rotation _returnvalue) "1.000000,1.000000,1.000000"))
  (Animation|PlayAnimMontage (Variables|Default|GetPlayerCharacter) "/Game/Skvt/Characters/Animations/Attacks/Att_BreakNeck_Montage.Att_BreakNeck_Montage" 1.0 "None")
  (bind _returnvalue_2 (Animation|PlayAnimMontage "/Game/Skvt/Characters/Animations/Attacks/Hit_BreakNeck_Montage.Hit_BreakNeck_Montage" 1.0 "None"))
  (Utilities|FlowControl|Delay _returnvalue_2)
  (Pawn|Components|CharacterMovement|SetMovementMode (Variables|/Script/Engine.Character|GetCharacterMovement (Variables|Default|GetPlayerCharacter)) "MOVE_Walking" 0))

(event Game|Damage|EventAnyDamage
  (params (Damage :type Float%20%28single-precision%29) (DamageType :type Damage%20Type%20Object%20Reference) (InstigatedBy :type Controller%20Object%20Reference) (DamageCauser :type Actor%20Object%20Reference))
  (Default|ProcessDamage (Variables|Default|GetBP_HealthComponent) Damage)
  (Animation|PlayAnimMontage "/Game/Skvt/Characters/Animations/Attacks/AM_Hit_punch.AM_Hit_punch" 1.0 "None"))

(event Collision|EventActorBeginOverlap
  (params (OtherActor :type Actor%20Object%20Reference)))

(event EventTick
  (params (DeltaSeconds :type Float%20%28single-precision%29)))

(event EventBeginPlay)

(event EventTriggerInteracting
  (params (Character :type BP%20Skvt%20Base%20Char%20Object%20Reference))
  (Variables|Default|SetPlayerCharacter Character)
  (CallFunction|Takedown false))

(fn ConstructionScript)

(fn GetAvailableInteractionAction
  (if (Variables|Default|GetIsDead)
    (return "NewEnumerator3")
    (else
      (return "NewEnumerator2"))))