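; BP_EMP is an EMP bomb actor that counts down, then disables or affects nearby electric actors.
; It triggers itself once, two seconds after BeginPlay, and updates a WB_EmpCountdown widget every second.
; At zero it draws a debug sphere and calls ApplyEMPEffect on overlapping BP_ElectricActors, hiding the widget in that loop.
; The construction script sizes the Sphere component to ImpactRadius.
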(event Custom|Trigger
  (if (not (Variables|Default|GetTriggered))
    (Variables|Default|SetTriggered true)
    (bind _aswb_emp_countdown (Utilities|Casting|CastToWB_EmpCountdown (UserInterface|GetWidget (Variables|Default|GetCountdownWidget))))
    (if (> (Variables|Default|GetCountdownValue) 0) :!label _label
      (bind _output_get (Variables|Default|SetCountdownValue (- (Variables|Default|GetCountdownValue) 1)))
      (Default|SetCountdownValue _aswb_emp_countdown _output_get)
      (Utilities|FlowControl|Delay 1.0)
      (goto _label)
      (else
        (Rendering|Debug|DrawDebugSphere (Transformation|GetWorldLocation (Variables|Default|GetBomb self)) (Variables|Default|GetImpactRadius) 30 "(R=1.000000,G=0.000000,B=0.054695,A=1.000000)" 5.0 2.0)
        (for _array_element (Collision|GetOverlappingActors self 0 :!class /Script/Engine.Actor)
          (bind _asbp_electric_actor (Utilities|Casting|CastToBP_ElectricActor _array_element))
          (Default|ApplyEMPEffect _asbp_electric_actor)
          (Rendering|SetVisibility (Variables|Default|GetCountdownWidget) false false))))))

(event EventBeginPlay
  (Utilities|FlowControl|Delay 2.0)
  (CallFunction|Trigger))

(event Collision|EventActorBeginOverlap
  (params (OtherActor :type Actor%20Object%20Reference)))

(event EventTick
  (params (DeltaSeconds :type Float%20%28single-precision%29)))

(fn ConstructionScript
  (Components|Sphere|SetSphereRadius (Variables|Default|GetSphere) (Variables|Default|GetImpactRadius) true))