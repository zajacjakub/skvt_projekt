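; EMP platform that sets off an electromagnetic pulse when a BP_SkvtBaseChar overlaps its trigger box.
; The pulse draws a debug sphere at the EMP bomb, gathers electric actors within ImpactRadius and calls ApplyEMPEffect on each.
; The construction script sizes the EMP collision sphere to the same radius.
; Two delay helper macros are defined but not used by the event graph.
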(event OnComponentBeginOverlap(Box)
  (params (OverlappedComponent :type Primitive%20Component%20Object%20Reference) (OtherActor :type Actor%20Object%20Reference) (OtherComp :type Primitive%20Component%20Object%20Reference) (OtherBodyIndex :type Integer) (bFromSweep :type Boolean) (SweepResult :type Hit%20Result%20Structure%20%28by%20ref%29))
  (Utilities|Casting|CastToBP_SkvtBaseChar OtherActor)
  (CallFunction|TriggertEMP))

(event Custom|TriggertEMP
  (Rendering|Debug|DrawDebugSphere (Transformation|GetWorldLocation (Variables|Default|GetEMP%20Bomb)) (Variables|Default|GetImpactRadius) 30 "(R=1.000000,G=0.000000,B=0.054695,A=1.000000)" 5.0 2.0)
  (bind _actors (CallFunction|GetElectricActorsinRadius (Transformation|GetWorldLocation (Variables|Default|GetEMP%20Bomb)) (Variables|Default|GetImpactRadius)))
  (for _array_element _actors
    (Default|ApplyEMPEffect _array_element)))

(event EventBeginPlay)

(event Collision|EventActorBeginOverlap
  (params (OtherActor :type Actor%20Object%20Reference)))

(event EventTick
  (params (DeltaSeconds :type Float%20%28single-precision%29)))

(fn ConstructionScript
  (Components|Sphere|SetSphereRadius (Variables|Default|GetEMPCollisionRadius) (Variables|Default|GetImpactRadius) true))