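; BP_Platform is a trigger actor that switches referenced actors on while something overlaps it and off when an overlap ends.
; Begin and end overlap loop over ActorsRef and send ToggleOnMessage to every entry implementing BPI_Electric, without filtering the overlapping actor or counting occupants.
; A leftover loop calling ToggleLight on LightsRef is unconnected and never runs.
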(event EventBeginPlay)

(event Collision|EventActorBeginOverlap
  (params (OtherActor :type Actor%20Object%20Reference))
  (for _array_element (Variables|Default|GetActorsRef)
    (if (Utilities|DoesObjectImplementInterface _array_element "/Game/Skvt/Blueprints/BPI_Electric.BPI_Electric_C")
      (Class|BPIElectric|Toggleon(Message) _array_element true))))

(event EventTick
  (params (DeltaSeconds :type Float%20%28single-precision%29)))

(event Collision|EventActorEndOverlap
  (params (OtherActor :type Actor%20Object%20Reference))
  (for _array_element (Variables|Default|GetActorsRef)
    (if (Utilities|DoesObjectImplementInterface _array_element "/Game/Skvt/Blueprints/BPI_Electric.BPI_Electric_C")
      (Class|BPIElectric|Toggleon(Message) _array_element false))))

(fn ConstructionScript)