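; BP_Doors is a door Blueprint that shows a prompt widget when the player character is near.
; Its Box overlap events respond only to BP_SkvtBaseChar, showing WidgetDorrUnlocked on entry and hiding it on exit.
; Entry checks the character's HasKey, but both branches show the same unlocked widget, so the key makes no difference.
; It contains no logic to open or unlock the door.
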(event OnComponentBeginOverlap(Box)
  (params (OverlappedComponent :type Primitive%20Component%20Object%20Reference) (OtherActor :type Actor%20Object%20Reference) (OtherComp :type Primitive%20Component%20Object%20Reference) (OtherBodyIndex :type Integer) (bFromSweep :type Boolean) (SweepResult :type Hit%20Result%20Structure%20%28by%20ref%29))
  (bind _asbp_skvt_base_char (Utilities|Casting|CastToBP_SkvtBaseChar OtherActor))
  (if (Variables|/Game/Skvt/Characters/BP_SkvtBaseChar.BP_SkvtBaseChar_C|GetHasKey _asbp_skvt_base_char)
    (Rendering|SetVisibility (Variables|Default|GetWidgetDorrUnlocked) true false)
    (else
      (Rendering|SetVisibility (Variables|Default|GetWidgetDorrUnlocked) true false))))

(event OnComponentEndOverlap(Box)
  (params (OverlappedComponent :type Primitive%20Component%20Object%20Reference) (OtherActor :type Actor%20Object%20Reference) (OtherComp :type Primitive%20Component%20Object%20Reference) (OtherBodyIndex :type Integer))
  (Utilities|Casting|CastToBP_SkvtBaseChar OtherActor)
  (Rendering|SetVisibility (Variables|Default|GetWidgetDorrUnlocked) false false)
  (Rendering|SetVisibility (Variables|Default|GetWidgetDorrUnlocked) false false))

(fn ConstructionScript)