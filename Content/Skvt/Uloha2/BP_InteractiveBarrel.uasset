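; Searchable barrel that a BP_SkvtBaseChar can interact with, ending either empty or with a key found.
; Capsule overlap stores the character and registers the barrel as its InteractableObject; end overlap clears InteractingCharacter and hides widgets.
; Search events drive a Status state machine, with the key result passed in on completion.
; While a character is stored, Tick shows the widget matching Status, with a delayed hide for finished searches.
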(event OnComponentBeginOverlap(Capsule)
  (params (OverlappedComponent :type Primitive%20Component%20Object%20Reference) (OtherActor :type Actor%20Object%20Reference) (OtherComp :type Primitive%20Component%20Object%20Reference) (OtherBodyIndex :type Integer) (bFromSweep :type Boolean) (SweepResult :type Hit%20Result%20Structure%20%28by%20ref%29))
  (bind _asbp_skvt_base_char (Utilities|Casting|CastToBP_SkvtBaseChar OtherActor))
  (Variables|Default|SetInteractingCharacter _asbp_skvt_base_char)
  (Variables|/Game/Skvt/Characters/BP_SkvtBaseChar.BP_SkvtBaseChar_C|SetInteractableObject (Variables|Default|GetInteractingCharacter) self))

(event OnComponentEndOverlap(Capsule)
  (params (OverlappedComponent :type Primitive%20Component%20Object%20Reference) (OtherActor :type Actor%20Object%20Reference) (OtherComp :type Primitive%20Component%20Object%20Reference) (OtherBodyIndex :type Integer))
  (Variables|Default|SetInteractingCharacter 0)
  (Variables|/Game/Skvt/Characters/BP_SkvtBaseChar.BP_SkvtBaseChar_C|SetInteractableObject (Variables|Default|GetInteractingCharacter) 0)
  (CallFunction|HideAllWidgets))

(event Custom|Start%20Search%20of%20barrel
  (Development|PrintString "Start Search")
  (if (Utilities|Enum|Equal(Enum) (Variables|Default|GetStatus) "NewEnumerator0")
    (Variables|Default|SetStatus "NewEnumerator1")))

(event Custom|Cancel%20Search%20of%20barrel
  (if (Utilities|Enum|Equal(Enum) (Variables|Default|GetStatus) "NewEnumerator1")
    (Variables|Default|SetStatus "NewEnumerator0")))

(event Custom|Start%20Searching
  (if (Utilities|Enum|Equal(Enum) (Variables|Default|GetStatus) "NewEnumerator0")
    (Variables|Default|SetStatus "NewEnumerator1")))

(event Custom|Stop%20Searching
  (if (Utilities|Enum|Equal(Enum) (Variables|Default|GetStatus) "NewEnumerator1")
    (Variables|Default|SetStatus "NewEnumerator0")))

(event Custom|Complete%20Search%20of%20a%20barrel
  (params (FoundKey :type Boolean))
  (if (Utilities|Enum|Equal(Enum) (Variables|Default|GetStatus) "NewEnumerator1")
    (if FoundKey
      (Variables|Default|SetStatus "NewEnumerator3")
      (else
        (Variables|Default|SetStatus "NewEnumerator2")))))

(event EventTick
  (params (DeltaSeconds :type Float%20%28single-precision%29))
  (Utilities|IsValid (Variables|Default|GetInteractingCharacter)
    (:Is%20Valid
      (bind _delay (CallFunction|ShowWidget))
      (if _delay
        (Utilities|FlowControl|Delay 2.0)
        (CallFunction|HideAllWidgets)))))

(fn ConstructionScript)

(fn ShowWidget
  (Development|PrintString (Utilities|String|EnumtoString (Variables|Default|GetStatus)))
  (CallFunction|HideAllWidgets)
  (switch Utilities|FlowControl|Switch|SwitchonEnum_InteractiveBarrelStatus (Variables|Default|GetStatus)
    (:NewEnumerator0
      (Rendering|SetVisibility (Variables|Default|GetWidget_Hint) true false)
      (Variables|Default|SetReturnBool false :!label _label))
    (:NewEnumerator1
      (Rendering|SetVisibility (Variables|Default|GetWidget_Searching) true false)
      (goto _label))
    (:NewEnumerator2
      (Rendering|SetVisibility (Variables|Default|GetWidget_NothingFound) true false)
      (Variables|Default|SetReturnBool true :!label _label_2))
    (:NewEnumerator3
      (Rendering|SetVisibility (Variables|Default|GetWidget_KeyFound) true false)
      (goto _label_2)))
  (return (Variables|Default|GetReturnBool)))

(fn HideAllWidgets
  (Rendering|SetVisibility (Variables|Default|GetWidget_Hint) false false))