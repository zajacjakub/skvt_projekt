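; BP_Doors is a locked door that the player character can open when holding a key.
; Overlapping its Box registers it as the BP_SkvtBaseChar's InteractableObject and shows a locked or unlocked widget based on HasKey.
; Leaving hides both widgets but still assigns the door as InteractableObject instead of clearing it.
; StartInteracting rechecks the key, hides the unlocked widget and plays a timeline that yaws the Door open.
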(event OnComponentBeginOverlap(Box)
  (params (OverlappedComponent :type Primitive%20Component%20Object%20Reference) (OtherActor :type Actor%20Object%20Reference) (OtherComp :type Primitive%20Component%20Object%20Reference) (OtherBodyIndex :type Integer) (bFromSweep :type Boolean) (SweepResult :type Hit%20Result%20Structure%20%28by%20ref%29))
  (bind _asbp_skvt_base_char (Utilities|Casting|CastToBP_SkvtBaseChar OtherActor))
  (Variables|/Game/Skvt/Characters/BP_SkvtBaseChar.BP_SkvtBaseChar_C|SetInteractable%20Object _asbp_skvt_base_char self)
  (if (Variables|/Game/Skvt/Characters/BP_SkvtBaseChar.BP_SkvtBaseChar_C|GetHasKey _asbp_skvt_base_char)
    (Rendering|SetVisibility (Variables|Default|GetWidgetDorrUnlocked) true false)
    (else
      (Rendering|SetVisibility (Variables|Default|GetWidgetDoorLocked) true false))))

(event OnComponentEndOverlap(Box)
  (params (OverlappedComponent :type Primitive%20Component%20Object%20Reference) (OtherActor :type Actor%20Object%20Reference) (OtherComp :type Primitive%20Component%20Object%20Reference) (OtherBodyIndex :type Integer))
  (bind _asbp_skvt_base_char (Utilities|Casting|CastToBP_SkvtBaseChar OtherActor))
  (Variables|/Game/Skvt/Characters/BP_SkvtBaseChar.BP_SkvtBaseChar_C|SetInteractable%20Object _asbp_skvt_base_char self)
  (Rendering|SetVisibility (Variables|Default|GetWidgetDorrUnlocked) false false)
  (Rendering|SetVisibility (Variables|Default|GetWidgetDoorLocked) false false))

(event Custom|Unlock%20The%20Door
  (bind _doortimer (Timeline|OpeningDoor Play)
    (:Update
      (Transformation|SetRelativeRotation (Variables|Default|GetDoor) (Math|Rotator|MakeRotator 0.0 0.0 (* _doortimer 9e+01)) false false))))

(event EventStartInteracting
  (params (Character :type BP%20Skvt%20Base%20Char%20Object%20Reference))
  (if (Variables|/Game/Skvt/Characters/BP_SkvtBaseChar.BP_SkvtBaseChar_C|GetHasKey Character)
    (Rendering|SetVisibility (Variables|Default|GetWidgetDorrUnlocked) false false)
    (CallFunction|UnlocktheDoor)))

(fn ConstructionScript)