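; BP_InteractiveBarrel is a searchable barrel that grants a key when it is the character's third searched barrel.
; Capsule overlap registers it as the BP_SkvtBaseChar's InteractableObject.
; Start, trigger and cancel events drive a Status enum from unsearched through searching to empty or key found, using the character's search counter.
; While a character is set, Tick shows the widget matching Status, with a delayed hide for results.
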(event OnComponentBeginOverlap(Capsule)
  (params (OverlappedComponent :type Primitive%20Component%20Object%20Reference) (OtherActor :type Actor%20Object%20Reference) (OtherComp :type Primitive%20Component%20Object%20Reference) (OtherBodyIndex :type Integer) (bFromSweep :type Boolean) (SweepResult :type Hit%20Result%20Structure%20%28by%20ref%29))
  (bind _asbp_skvt_base_char (Utilities|Casting|CastToBP_SkvtBaseChar OtherActor))
  (Variables|Default|SetInteractingCharacter _asbp_skvt_base_char)
  (Variables|/Game/Skvt/Characters/BP_SkvtBaseChar.BP_SkvtBaseChar_C|SetInteractable%20Object (Variables|Default|GetInteractingCharacter) self))

(event OnComponentEndOverlap(Capsule)
  (params (OverlappedComponent :type Primitive%20Component%20Object%20Reference) (OtherActor :type Actor%20Object%20Reference) (OtherComp :type Primitive%20Component%20Object%20Reference) (OtherBodyIndex :type Integer))
  (Variables|Default|SetInteractingCharacter 0)
  (Utilities|IsValid (Variables|Default|GetInteractingCharacter)
    (:Is%20Valid
      (Variables|/Game/Skvt/Characters/BP_SkvtBaseChar.BP_SkvtBaseChar_C|SetInteractable%20Object (Variables|Default|GetInteractingCharacter) 0))
    (:Is%20Not%20Valid
      _))
  (CallFunction|HideAllWidgets))

(event EventTick
  (params (DeltaSeconds :type Float%20%28single-precision%29))
  (Utilities|IsValid (Variables|Default|GetInteractingCharacter)
    (:Is%20Valid
      (bind _delay (CallFunction|ShowWidget))
      (if _delay
        (Utilities|FlowControl|Delay 2.0)
        (CallFunction|HideAllWidgets)))))

(event EventTriggerInteracting
  (params (Character :type BP%20Skvt%20Base%20Char%20Object%20Reference))
  (if (Utilities|Enum|Equal(Enum) (Variables|Default|GetStatus) "NewEnumerator1")
    (bind _output_get (Variables|/Game/Skvt/Characters/BP_SkvtBaseChar.BP_SkvtBaseChar_C|SetNumberOfBarrelSearched Character (+ (Variables|/Game/Skvt/Characters/BP_SkvtBaseChar.BP_SkvtBaseChar_C|GetNumberOfBarrelSearched Character) 1)))
    (if (== _output_get 3)
      (Variables|Default|SetStatus "NewEnumerator3")
      (Variables|/Game/Skvt/Characters/BP_SkvtBaseChar.BP_SkvtBaseChar_C|SetHasKey (Variables|Default|GetInteractingCharacter) true)
      (else
        (Variables|Default|SetStatus "NewEnumerator2")))))

(event EventCancelInteracting
  (params (Character :type BP%20Skvt%20Base%20Char%20Object%20Reference))
  (if (Utilities|Enum|Equal(Enum) (Variables|Default|GetStatus) "NewEnumerator1")
    (Variables|Default|SetStatus "NewEnumerator0")))

(event EventStartInteracting
  (params (Character :type BP%20Skvt%20Base%20Char%20Object%20Reference))
  (if (Utilities|Enum|Equal(Enum) (Variables|Default|GetStatus) "NewEnumerator0")
    (Variables|Default|SetStatus "NewEnumerator1")))

(fn ConstructionScript)

(fn ShowWidget
  (CallFunction|HideAllWidgets)
  (switch Utilities|FlowControl|Switch|SwitchonEnum_InteractiveBarrelStatus (Variables|Default|GetStatus)
    (:NewEnumerator0
      (Rendering|SetVisibility (Variables|Default|GetWidget_Hint) true false)
      (Variables|Default|SetReturnBool false :!label _label))
    (:NewEnumerator1
      (Rendering|SetVisibility (Variables|Default|GetWidget_Searching) true false)
      (goto _label))
    (:NewEnumerator2
      (Rendering|SetVisibility (Variables|Default|GetWidget_NothingFound) true false)
      (Variables|Default|SetReturnBool true :!label _label_2))
    (:NewEnumerator3
      (Rendering|SetVisibility (Variables|Default|GetWidget_KeyFound) true false)
      (goto _label_2)))
  (return (Variables|Default|GetReturnBool)))

(fn HideAllWidgets
  (Rendering|SetVisibility (Variables|Default|GetWidget_Hint) false false))