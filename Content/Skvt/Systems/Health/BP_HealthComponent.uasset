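; BP_HealthComponent is a health component that tracks current and maximum health and signals death.
; ProcessDamage subtracts damage through UpdateHealth, which clamps Health between zero and MaxHealth and calls OnDeath whenever the result is zero, with no guard against repeat calls.
; UpdateMaxHealth sets a new maximum and refills Health to it, while IsDead reports whether Health is zero.
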(event EventBeginPlay)

(event EventTick
  (params (DeltaSeconds :type Float%20%28single-precision%29)))

(fn UpdateHealth
  (params (NewHealth :type Float%20%28double-precision%29))
  (bind _output_get (Variables|Default|SetHealth (Math|Float|Clamp(Float) NewHealth 0.0 (Variables|Default|GetMaxHealth))))
  (if (== _output_get 0.0)
    (Default|CallOnDeath)))

(fn UpdateMaxHealth
  (params (NewMaxHealth :type Float%20%28double-precision%29))
  (bind _output_get (Variables|Default|SetMaxHealth NewMaxHealth))
  (Variables|Default|SetHealth _output_get))

(fn ProcessDamage
  (params (DamageDealt :type Float%20%28double-precision%29))
  (CallFunction|UpdateHealth (- (Variables|Default|GetHealth) DamageDealt)))

(fn IsDead
  (return (== (Variables|Default|GetHealth) 0.0)))